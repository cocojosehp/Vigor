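; Interactive double door that the player swings open or shut with F while overlapping its collision component, which toggles the actor's input.
; Two parallel F handlers drive the Open_Left and Open_Right timelines, each setting the yaw of its door mesh.
; They share IsMoving, which gates the sound, and ClosedDoor, which picks Play or Reverse.
; FlipFlops on timeline finish set ClosedDoor, which despite its name selects Reverse when true.
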(event `self.CollisionComp.OnComponentBeginOverlap`
  (params (OverlappedComponent :type "PrimitiveComponent Object Reference") (OtherActor :type "Actor Object Reference") (OtherComp :type "PrimitiveComponent Object Reference") (OtherBodyIndex :type Integer) (bFromSweep :type Boolean) (SweepResult :type "HitResult Structure (by ref)"))
  (`self.EnableInput` (`GameplayStatics.GetPlayerController` 0)))

(event `self.CollisionComp.OnComponentEndOverlap`
  (params (OverlappedComponent :type "PrimitiveComponent Object Reference") (OtherActor :type "Actor Object Reference") (OtherComp :type "PrimitiveComponent Object Reference") (OtherBodyIndex :type Integer))
  (`self.DisableInput` (`GameplayStatics.GetPlayerController` 0)))

(event `Key|F`
  (params (Key :type "Key Structure"))
  (:`Pressed`
    (if (`self.Closed Door`)
      (if (`self.Is Moving?`)
        (bind (_direction _opendoor) (`Timeline|Open_Left` :!via `Reverse` :!label _label)
          (:`Update`
            (`SceneComponent.K2_SetRelativeRotation` (`self.DoorMesh_L`) (`KismetMathLibrary.MakeRotator` 0.0 0.0 _opendoor) false false))
          (:`Finished`
            (set `self.Is Moving?` false)
            (`/Engine/EditorBlueprintResources/StandardMacros.FlipFlop`
              (:`A`
                (set `self.Closed Door` true))
              (:`B`
                (set `self.Closed Door` false)))))
        (else
          (set `self.Is Moving?` true)
          (`GameplayStatics.SpawnSoundAtLocation` null (`self.K2_GetActorLocation`))
          (goto _label :!via `Reverse`)))
      (elif (`self.Is Moving?`)
        (goto _label)
        (else
          (set `self.Is Moving?` true)
          (`GameplayStatics.SpawnSoundAtLocation` null (`self.K2_GetActorLocation`))
          (goto _label))))))

(event `Key|F`
  (params (Key :type "Key Structure"))
  (:`Pressed`
    (if (`self.Closed Door`)
      (if (`self.Is Moving?`)
        (bind (_direction _opendoor) (`Timeline|Open_Right` :!via `Reverse` :!label _label_2)
          (:`Update`
            (`SceneComponent.K2_SetRelativeRotation` (`self.DoorMesh_R`) (`KismetMathLibrary.MakeRotator` 0.0 0.0 _opendoor) false false))
          (:`Finished`
            (set `self.Is Moving?` false)
            (`/Engine/EditorBlueprintResources/StandardMacros.FlipFlop`
              (:`A`
                (set `self.Closed Door` true))
              (:`B`
                (set `self.Closed Door` false)))))
        (else
          (set `self.Is Moving?` true)
          (`GameplayStatics.SpawnSoundAtLocation` null (`self.K2_GetActorLocation`))
          (goto _label_2 :!via `Reverse`)))
      (elif (`self.Is Moving?`)
        (goto _label_2)
        (else
          (set `self.Is Moving?` true)
          (`GameplayStatics.SpawnSoundAtLocation` null (`self.K2_GetActorLocation`))
          (goto _label_2))))))

(fn `UserConstructionScript`)